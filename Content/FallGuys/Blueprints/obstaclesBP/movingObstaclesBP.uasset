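; A moving obstacle actor that takes one of three random meshes and travels along a referenced spline.
; On BeginPlay it picks the mesh and plays a timeline, whose alpha maps to distance along the spline to set world location and rotation.
; A six-second Delay fed by the timeline's Update loops back to pick a new mesh and restart the run from the beginning.
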(event `self.ReceiveBeginPlay`
  (bind _returnvalue (`KismetMathLibrary.Lerp` 0.0 (`SplineComponent.GetSplineLength` (`/Game/FallGuys/Blueprints/obstaclesBP/splineActorBP.Spline` (`self.spline`))) (`self.alpha`)))
  (switch `int` (`KismetMathLibrary.RandomIntegerInRange` 0 2) :!label _label
    (:`0`
      (`StaticMeshComponent.SetStaticMesh` (`self.StaticMesh`) "/Game/FallGuys/Blueprints/obstaclesBP/obstacle1.obstacle1")
      (bind (_direction _newtrack_0) (`Timeline|Timeline_0` :!via `PlayFromStart` :!label _label_2)
        (:`Update`
          (set `self.alpha` _newtrack_0)
          (`self.K2_SetActorLocationAndRotation` (`SplineComponent.GetLocationAtDistanceAlongSpline` (`/Game/FallGuys/Blueprints/obstaclesBP/splineActorBP.Spline` (`self.spline`)) _returnvalue "World") (`SplineComponent.GetRotationAtDistanceAlongSpline` (`/Game/FallGuys/Blueprints/obstaclesBP/splineActorBP.Spline` (`self.spline`)) _returnvalue "World"))
          (`KismetSystemLibrary.Delay` 6.0)
          (goto _label))))
    (:`1`
      (`StaticMeshComponent.SetStaticMesh` (`self.StaticMesh`) "/Game/FallGuys/Blueprints/obstaclesBP/obstacle2.obstacle2")
      (goto _label_2 :!via `PlayFromStart`))
    (:`2`
      (`StaticMeshComponent.SetStaticMesh` (`self.StaticMesh`) "/Game/FallGuys/Blueprints/obstaclesBP/obstacle3.obstacle3")
      (goto _label_2 :!via `PlayFromStart`))))

(fn `UserConstructionScript`)