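; GoalArea is the finish-zone actor in a Fall Guys-style game that registers characters reaching the goal.
; On overlap it casts the actor to ThirdPersonCharacter or AICharacter and sets its ReachedGoal flag.
; It then writes a point into PointsToAdd at that character's PlayerID and sets End to true.
; Nodes that zero the HUD time are left unconnected and never run.
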(event `self.ReceiveActorBeginOverlap`
  (params (OtherActor :type "Actor Object Reference"))
  (if (== (`GameplayStatics.GetObjectClass` OtherActor) "/Game/ThirdPersonBP/Blueprints/ThirdPersonCharacter.ThirdPersonCharacter_C")
    (bind _asthird_person_character (cast `/Game/ThirdPersonBP/Blueprints/ThirdPersonCharacter` OtherActor))
    (set `/Game/ThirdPersonBP/Blueprints/ThirdPersonCharacter.ReachedGoal` true _asthird_person_character)
    (`KismetArrayLibrary.Array_Set` (`self.PointsToAdd`) (`/Game/ThirdPersonBP/Blueprints/ThirdPersonCharacter.PlayerID` _asthird_person_character) 1)
    (set `self.End` true)
    (else
      (bind _asaicharacter (cast `/Game/ThirdPersonBP/Blueprints/AICharacter` OtherActor))
      (set `/Game/ThirdPersonBP/Blueprints/AICharacter.ReachedGoal` true _asaicharacter)
      (`KismetArrayLibrary.Array_Set` (`self.PointsToAdd`) (`/Game/ThirdPersonBP/Blueprints/AICharacter.PlayerID` _asaicharacter) 1)
      (set `self.End` true))))

(fn `UserConstructionScript`)