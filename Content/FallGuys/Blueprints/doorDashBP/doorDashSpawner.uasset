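; Spawner for a row of doors in a Fall Guys-style Door Dash obstacle.
; On BeginPlay it spawns three doors at even intervals along world X, starting from its Scene component's world location.
; One randomly chosen slot gets a FakeDoor and the other two get RealDoors, so the layout can vary each time play begins.
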(event `self.ReceiveBeginPlay`
  (set `self.random` (`KismetMathLibrary.RandomIntegerInRange` 0 2))
  (for _index (range 3)
    (set `self.location` (+ (`KismetMathLibrary.MakeVector` (* _index 400.0)) (`SceneComponent.K2_GetComponentLocation` (`self.Scene`))))
    (if (== _index (`self.random`))
      (`|SpawnActorFromClass` "/Game/FallGuys/Blueprints/doorDashBP/fakeDoor.fakeDoor_C" (`KismetMathLibrary.MakeTransform` (`self.location`)) "Undefined" "OverrideRootScale" null null)
      (else
        (`|SpawnActorFromClass` "/Game/FallGuys/Blueprints/doorDashBP/realDoor.realDoor_C" (`KismetMathLibrary.MakeTransform` (`self.location`)) "Undefined" "OverrideRootScale" null null)))))

(fn `UserConstructionScript`)