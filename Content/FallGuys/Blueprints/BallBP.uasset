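; BallBP is a randomly coloured physics ball that acts as a self-replicating launcher.
; On BeginPlay it stores its start transform and tints a dynamic material created in the construction script.
; After a random delay of several seconds it spawns another BallBP at that transform, then applies an impulse to its own Ball component.
; Each new ball repeats the cycle, and this Blueprint never destroys old ones.
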(event `self.ReceiveBeginPlay`
  (set `self.InitialTransform` (`self.GetTransform`))
  (`self.RandomColour`)
  (`self.SpawnBall`))

(event `RandomColour`
  ;[1 1 1] Set random colour
  (`MaterialInstanceDynamic.SetVectorParameterValue` (`self.DynamicMaterial`) "Color" (`KismetMathLibrary.MakeColor` (`KismetMathLibrary.RandomFloatInRange` 0.0 1.0) (`KismetMathLibrary.RandomFloatInRange` 0.0 1.0) (`KismetMathLibrary.RandomFloatInRange` 0.0 1.0))))

(event `SpawnBall`
  (`KismetSystemLibrary.Delay` (`KismetMathLibrary.RandomFloatInRange` 5.5 7.0))
  (bind _returnvalue (`|SpawnActorFromClass` "BallBP_C" (`self.InitialTransform`) "Undefined" "OverrideRootScale" null null))
  (`self.K2_SetActorTransform` _returnvalue (`self.InitialTransform`) false false)
  (`PrimitiveComponent.AddImpulse` (`self.Ball`) (1000.0 5000.0 1000.0) "None" false))

(fn `Decrement`
  (set `self.TimerValue` (- (`self.TimerValue`) 1)))

(fn `UserConstructionScript`
  (bind _returnvalue (`PrimitiveComponent.CreateDynamicMaterialInstance` (`self.Ball`) 0 null "None"))
  (set `self.DynamicMaterial` _returnvalue))