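; Hexagon floor tile actor for a Fall Guys-style game that vanishes after a character steps on it.
; The Box overlap accepts ThirdPersonCharacter or AICharacter, with both paths feeding a single DoOnce so the tile triggers only once.
; It drops slightly, swaps the StaticMesh material after a short delay, then destroys itself after another.
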(event `self.Box.OnComponentBeginOverlap`
  (params (OverlappedComponent :type "PrimitiveComponent Object Reference") (OtherActor :type "Actor Object Reference") (OtherComp :type "PrimitiveComponent Object Reference") (OtherBodyIndex :type Integer) (bFromSweep :type Boolean) (SweepResult :type "HitResult Structure (by ref)"))
  (if (== (`GameplayStatics.GetObjectClass` OtherActor) "/Game/ThirdPersonBP/Blueprints/ThirdPersonCharacter.ThirdPersonCharacter_C")
    (cast `/Game/ThirdPersonBP/Blueprints/ThirdPersonCharacter` OtherActor)
    (else
      (cast `/Game/ThirdPersonBP/Blueprints/AICharacter` OtherActor)))
  (`/Engine/EditorBlueprintResources/StandardMacros.DoOnce` false
    (:`Completed`
      (`self.K2_AddActorLocalOffset` (0.0 0.0 -5.0))
      (`KismetSystemLibrary.Delay` 0.2)
      (`PrimitiveComponent.SetMaterial` (`self.StaticMesh`) 0 "/Game/InfinityBladeGrassLands/Maps/LevelContent/Architecture/M_1Meter_01.M_1Meter_01")
      (`KismetSystemLibrary.Delay` 0.3)
      (`self.K2_DestroyActor`))))

(fn `UserConstructionScript`)