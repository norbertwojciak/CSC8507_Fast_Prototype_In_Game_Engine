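; Spawner actor in the Fall Guys hexagon blueprints that builds a line of alternating Hexaspawn1 and Hexaspawn2 actors when play begins.
; A loop steps at even spacing along world X from the Scene component's location, spawning one actor per step.
; A FlipFlop inside the loop switches between the two classes on each iteration.
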(event `self.ReceiveBeginPlay`
  (for _index (range 11)
    (set `self.location` (+ (`SceneComponent.K2_GetComponentLocation` (`self.Scene`)) (`KismetMathLibrary.MakeVector` (* _index 150.0))))
    (`/Engine/EditorBlueprintResources/StandardMacros.FlipFlop`
      (:`A`
        (`|SpawnActorFromClass` "/Game/FallGuys/Blueprints/hexagonBP/hexaspawn1.hexaspawn1_C" (`KismetMathLibrary.MakeTransform` (`self.location`)) "Undefined" "OverrideRootScale" null null))
      (:`B`
        (`|SpawnActorFromClass` "/Game/FallGuys/Blueprints/hexagonBP/hexaspawn2.hexaspawn2_C" (`KismetMathLibrary.MakeTransform` (`self.location`)) "Undefined" "OverrideRootScale" null null)))))

(fn `UserConstructionScript`)